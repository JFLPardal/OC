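; Player-controllable character that moves from axis input and detects interactable actors around it.
; MoveForward and MoveToTheSide each overwrite one component of the capsule's facing vector to rotate it, then add movement along the capsule's forward vector, ignoring the passed direction.
; An InteractableVolume query reports whether another interactable besides the held one is in range.
; Overlap handlers are bound, but their debug prints are disconnected.
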(event `self.ReceiveBeginPlay`)

(event `InputAxis|MoveToTheSide`
  (params (AxisValue :type "Float (single-precision)"))
  (bind _returnvalue_x (`KismetMathLibrary.BreakVector` (`KismetMathLibrary.Conv_RotatorToVector` (`SceneComponent.K2_GetComponentRotation` (`self.CapsuleComponent`)))))
  (if (or (> AxisValue 0.1) (< AxisValue -0.1))
    ;[1 1 1] tentativa com rotationFromXVecot
    (`SceneComponent.K2_SetWorldRotation` (`self.CapsuleComponent`) (`KismetMathLibrary.Conv_VectorToRotator` (`KismetMathLibrary.MakeVector` _returnvalue_x AxisValue)) false false)
    (`self.UpdateMovementBasedOnInput` (`KismetMathLibrary.Conv_RotatorToVector` (`SceneComponent.K2_GetComponentRotation` (`self.CapsuleComponent`))) :!label _label)
    (else
      ;[1 1 1] tentativa com rotationFromXVecot
      (`SceneComponent.K2_SetWorldRotation` (`self.CapsuleComponent`) (`KismetMathLibrary.Conv_VectorToRotator` (`KismetMathLibrary.Conv_RotatorToVector` (`SceneComponent.K2_GetComponentRotation` (`self.CapsuleComponent`)))) false false :!label _label_2))))

(event `InputAxis|MoveForward`
  (params (AxisValue :type "Float (single-precision)"))
  (bind (_returnvalue_x _returnvalue_y) (`KismetMathLibrary.BreakVector` (`KismetMathLibrary.Conv_RotatorToVector` (`SceneComponent.K2_GetComponentRotation` (`self.CapsuleComponent`)))))
  (if (or (> AxisValue 0.1) (< AxisValue -0.1))
    ;[1 1 1] tentativa com rotationFromXVecot
    (`SceneComponent.K2_SetWorldRotation` (`self.CapsuleComponent`) (`KismetMathLibrary.Conv_VectorToRotator` (`KismetMathLibrary.MakeVector` AxisValue _returnvalue_y)) false false)
    (goto _label)
    (else
      (goto _label_2))))

(event `self.InteractableVolume.OnComponentBeginOverlap`
  (params (OverlappedComponent :type "PrimitiveComponent Object Reference") (OtherActor :type "Actor Object Reference") (OtherComp :type "PrimitiveComponent Object Reference") (OtherBodyIndex :type Integer) (bFromSweep :type Boolean) (SweepResult :type "HitResult Structure (by ref)"))
  ;[1 1 1] nukeable as these are only debugging functions
  (`self.OnOverlapBegin` OtherActor))

(event `self.InteractableVolume.OnComponentEndOverlap`
  (params (OverlappedComponent :type "PrimitiveComponent Object Reference") (OtherActor :type "Actor Object Reference") (OtherComp :type "PrimitiveComponent Object Reference") (OtherBodyIndex :type Integer))
  ;[1 1 1] nukeable as these are only debugging functions
  (`self.OnOverlapEnd` OtherActor))

(fn `Has Other Interactable in Radius`
  (returns (ReturnValue :type Boolean))
  (return (> (`KismetArrayLibrary.Array_Length` (`PrimitiveComponent.GetOverlappingActors` (`self.InteractableVolume`) "/Script/OC.InteractableActor")) 1)))

(fn `OnOverlapBegin`
  (params (OtherActor :type "Object Object Reference")))

(fn `OnOverlapEnd`
  (params (OtherActor :type "Object Object Reference")))

(fn `UpdateMovementBasedOnInput`
  (params (NewWorldDirection :type "Vector Structure"))
  (`self.AddMovementInput` (`SceneComponent.GetForwardVector` (`self.CapsuleComponent`))))

(fn `UserConstructionScript`)